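; Actor Blueprint that demonstrates functions by offsetting its own location and rotation.
; On BeginPlay, AddLocationOffset adds the LocationOffset variable to the actor's location and returns the new position, which is printed on screen.
; AddOctorRotation combines the current rotation with RotationOffset, applies it and prints the result, but nothing in this Blueprint calls it.
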(event EventBeginPlay
  (bind _newlocation (CallFunction|AddLocationOffset (Transformation|GetActorLocation)))
  (Development|PrintString (Utilities|String|ToString(Vector) _newlocation) true true "(R=1.000000,G=0.000000,B=0.029831,A=1.000000)" 1e+01))

(fn ConstructionScript)

(fn AddLocationOffset
  (params (ActualLocation :type Vector))
  (bind _locationoffset (Variables|Default|GetLocationOffset))
  (bind _returnvalue (+ ActualLocation _locationoffset))
  (Transformation|SetActorLocation _returnvalue false false)
  (return _returnvalue))

(fn AddOctorRotation
  (bind _returnvalue (Transformation|GetActorRotation))
  (bind _rotationoffset (Variables|Default|GetRotationOffset))
  (bind _returnvalue_2 (Math|Rotator|CombineRotators _returnvalue _rotationoffset))
  (Transformation|SetActorRotation _returnvalue_2)
  (Development|PrintString (Utilities|String|ToString(Rotator) _returnvalue_2)))