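; Demo Blueprint that uses a Sequence node on BeginPlay to move a Sphere component in printed, numbered stages.
; The first branch prints and raises the sphere, then the second branch immediately prints and raises it again.
; The second branch then waits on a Delay before printing a final message and shifting the sphere sideways along Y.
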(event EventBeginPlay
  (Utilities|FlowControl|Sequence
    (:then_0
      (Development|PrintString "Parte1")
      (Transformation|AddLocalOffset (Variables|Default|GetSphere) "0.000000,0.000000,100.000000" false false))
    (:then_1
      (Development|PrintString "Parte2")
      (Transformation|AddLocalOffset (Variables|Default|GetSphere) "0.000000,0.000000,100.000000" false false)
      (Utilities|FlowControl|Delay 5.0)
      (Development|PrintString "Parte3")
      (Transformation|AddLocalOffset (Variables|Default|GetSphere) "0.000000,200.000000,0.000000" false false))))

(fn ConstructionScript)