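; 005_Events is a Blueprint that keeps a coin count and prints it on screen, exercising input, overlap and custom events.
; When a Pawn overlaps the actor, it calls the AddCoins custom event to increment Coins, then CoinsPrint to display the total.
; Pressing Z also prints the current count; BeginPlay, Tick and the construction script are empty.
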(event Custom|AddCoins
  ;[0.15 0.15 0.15 0.5] Custom Event
  (Variables|Default|SetCoins (+ (Variables|Default|GetCoins) 1)))

(event Custom|CoinsPrint
  ;[0.15 0.15 0.15 0.5] Custom Event
  (Development|PrintString (Utilities|String|ToString(Integer) (Variables|Default|GetCoins))))

(event EventBeginPlay)

(event Collision|EventActorBeginOverlap
  (params (OtherActor :type Actor%20Object%20Reference))
  ;[0.15 0.15 0.15 0.5] Custom Event
  (Utilities|Casting|CastToPawn OtherActor)
  (CallFunction|AddCoins)
  (CallFunction|CoinsPrint))

(event EventTick
  (params (DeltaSeconds :type Float%20%28single-precision%29)))

(event Input|KeyboardEvents|Z
  (params (Key :type Key%20Structure :default "None"))
  (:Pressed
    (Development|PrintString (Utilities|String|ToString(Integer) (Variables|Default|GetCoins)))))

(fn ConstructionScript)