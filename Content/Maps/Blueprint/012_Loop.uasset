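; Tutorial-style Blueprint that demonstrates loop nodes by printing to the screen.
; On BeginPlay, a For Each loop prints every element of the Name array, then "Fine!".
; Disconnected examples show While, For, and breakable For and For Each loops, driven by LoopSteps, WhileLoopTF and LoopBreakeStep.
; These examples never run, and the construction script is empty.
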(event Custom|BreakLoop
  ;[0.15 0.15 0.15 0.5] ForLoop
  (bind _index (Utilities|FlowControl|ForLoopwithBreak 0 (Variables|Default|GetLoopSteps)) ; enters at Break
    (:LoopBody
      (if (> _index (Variables|Default|GetLoopBreakeStep))
        (CallFunction|BreakLoop)
        (else
          (Development|PrintString (Utilities|String|Append "Step" (Utilities|String|ToString(Integer) _index)) true true "(R=0.000000,G=0.660000,B=1.000000,A=1.000000)" 1e+01))))
    (:Completed
      (Development|PrintString "Fine!" true true "(R=0.000000,G=0.660000,B=1.000000,A=1.000000)" 3.0))))

(event EventBeginPlay
  ;[0.15 0.15 0.15 0.5] For Each Loop
  (for _array_element (Variables|Default|GetName)
    (Development|PrintString _array_element true true "(R=0.000000,G=0.660000,B=1.000000,A=1.000000)" 1e+01))
  (Development|PrintString "Fine!" true true "(R=0.000000,G=0.660000,B=1.000000,A=1.000000)" 1e+01))

(fn ConstructionScript)