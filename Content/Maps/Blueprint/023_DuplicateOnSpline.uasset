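; Spline placement Blueprint that duplicates a chosen mesh along a spline as instanced static meshes, built in the Construction Script.
; Spacing comes from the mesh's X bounds plus an offset, and spline length divided by it sets the count.
; Each instance faces the next distance sample, with optional per-axis random offsets to position, rotation and scale.
; The randomness is unseeded, so results vary whenever construction reruns.
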(event EventBeginPlay)

(event Collision|EventActorBeginOverlap
  (params (OtherActor :type Actor%20Object%20Reference)))

(event EventTick
  (params (DeltaSeconds :type Float%20%28single-precision%29)))

(fn ConstructionScript
  (bind _placedmesh (Variables|Default|GetPlacedMesh))
  (bind _returnvalue (StaticMesh|GetBoundingBox _placedmesh))
  (Components|StaticMesh|SetStaticMesh (Variables|Default|GetInstancedStaticMesh) _placedmesh)
  (bind _output_get (Variables|Default|SetSpacing (+ (.x (- (.max _returnvalue) (.min _returnvalue))) (Variables|Default|GetOffset))))
  (bind _output_get_2 (Variables|Default|SetInstanceNumber (Math|Float|Floor (/ (Spline|GetSplineLength (Variables|Default|GetSpline)) _output_get))))
  (for _index (range 0 _output_get_2)
    (Components|InstancedStaticMesh|AddInstance (Variables|Default|GetInstancedStaticMesh) (Math|Transform|MakeTransform (.location (Math|Transform|MakeTransform (CallFunction|AddRandomPosition (CallFunction|GetLocationatIndex _index)) (CallFunction|AddRandomRotation (Math|Rotator|MakeRotfromX (- (CallFunction|GetLocationatIndex (+ _index 1)) (CallFunction|GetLocationatIndex _index)))))) (.rotation (Math|Transform|MakeTransform (CallFunction|AddRandomPosition (CallFunction|GetLocationatIndex _index)) (CallFunction|AddRandomRotation (Math|Rotator|MakeRotfromX (- (CallFunction|GetLocationatIndex (+ _index 1)) (CallFunction|GetLocationatIndex _index)))))) (CallFunction|AddRandomScale (.scale (Math|Transform|MakeTransform (CallFunction|AddRandomPosition (CallFunction|GetLocationatIndex _index)) (CallFunction|AddRandomRotation (Math|Rotator|MakeRotfromX (- (CallFunction|GetLocationatIndex (+ _index 1)) (CallFunction|GetLocationatIndex _index)))))))) false)))

(fn GetLocationatIndex
  (params (A :type Integer))
  (return (Spline|GetLocationatDistanceAlongSpline (Variables|Default|GetSpline) (* A (Variables|Default|GetSpacing)) "Local")))

(fn AddRandomRotation
  (params (Rotation :type Rotator))
  (bind _returnvalue (CallFunction|RandomRotation))
  (bind _rotateaxis (Variables|Default|GetRotateAxis))
  (bind (_bx _by _bz) (Utilities|Struct|BreakFilterOptionPerAxis _rotateaxis))
  (return (Math|Rotator|MakeRotator (select _bx (+ (.roll Rotation) _returnvalue) (.roll Rotation)) (select _by (+ (.pitch Rotation) _returnvalue) (.pitch Rotation)) (select _bz (+ (.yaw Rotation) _returnvalue) (.yaw Rotation)))))

(fn RandomRotation
  (bind _randomrotationunit (Variables|Default|GetRandomRotationUnit))
  (bind (_min _max) (Utilities|Struct|BreakFloatInterval _randomrotationunit))
  (return (Math|Random|RandomFloatinRange _min _max)))

(fn AddRandomScale
  (params (Scale :type Vector))
  (bind _returnvalue (CallFunction|RandomScale))
  (bind _scaleaxis (Variables|Default|GetScaleAxis))
  (bind (_bx _by _bz) (Utilities|Struct|BreakFilterOptionPerAxis _scaleaxis))
  (return (Math|Vector|MakeVector (select _bx (+ (.x Scale) _returnvalue) (.x Scale)) (select _by (+ (.y Scale) _returnvalue) (.y Scale)) (select _bz (+ (.z Scale) _returnvalue) (.z Scale)))))

(fn RandomScale
  (bind _randomscaleunit (Variables|Default|GetRandomScaleUnit))
  (bind (_min _max) (Utilities|Struct|BreakFloatInterval _randomscaleunit))
  (return (Math|Random|RandomFloatinRange _min _max)))

(fn AddRandomPosition
  (params (Position :type Vector))
  (bind _returnvalue (CallFunction|RandomPosition))
  (bind _positionaxis (Variables|Default|GetPositionAxis))
  (bind (_bx _by _bz) (Utilities|Struct|BreakFilterOptionPerAxis _positionaxis))
  (return (Math|Vector|MakeVector (select _bx (+ (.x Position) _returnvalue) (.x Position)) (select _by (+ (.y Position) _returnvalue) (.y Position)) (select _bz (+ (.z Position) _returnvalue) (.z Position)))))

(fn RandomPosition
  (bind _randompositionunit (Variables|Default|GetRandomPositionUnit))
  (bind (_min _max) (Utilities|Struct|BreakFloatInterval _randompositionunit))
  (return (Math|Random|RandomFloatinRange _min _max)))