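; Example actor Blueprint that uses a MeshList enumeration to pick which primitive mesh it shows: cube, sphere, cylinder or cone.
; The Construction Script switches on MeshList and makes the matching mesh component visible, without propagating to children.
; BeginPlay is empty, and a disconnected branch would print an Italian message saying whether the selection is a cube.
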(event EventBeginPlay)

(fn ConstructionScript
  (switch Utilities|FlowControl|Switch|SwitchonE_Mesh (Variables|Default|GetMesh%20List)
    (:NewEnumerator0
      (Rendering|SetVisibility (Variables|Default|GetCube) true false))
    (:NewEnumerator1
      (Rendering|SetVisibility (Variables|Default|GetSphere) true false))
    (:NewEnumerator2
      (Rendering|SetVisibility (Variables|Default|GetCylinder) true false))
    (:NewEnumerator3
      (Rendering|SetVisibility (Variables|Default|GetCone) true false))))