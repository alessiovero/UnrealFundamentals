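; Example Actor Blueprint that demonstrates basic arithmetic operators on two variables, Value1 and Value2.
; On BeginPlay it computes their sum, difference, product and quotient, appends them into one labeled string and shows it with a long-duration Print String.
; The Construction Script is empty.
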(event EventBeginPlay
  (bind _value_1 (Variables|Default|GetValue_1))
  (bind _value_2 (Variables|Default|GetValue_2))
  (Development|PrintString (Utilities|String|Append "Add = " (Utilities|String|ToString(Float) (+ _value_1 _value_2)) " 
Subtract = " (Utilities|String|ToString(Float) (- _value_1 _value_2)) " 
Multiply = " (Utilities|String|ToString(Float) (* _value_1 _value_2)) " 
Divide = " (Utilities|String|ToString(Float) (/ _value_1 _value_2))) true true "(R=0.000000,G=0.660000,B=1.000000,A=1.000000)" 2e+01))

(fn ConstructionScript)