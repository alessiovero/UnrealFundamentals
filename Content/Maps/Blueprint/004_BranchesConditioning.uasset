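; Demo actor Blueprint that shows conditional branching on a comparison of two variables.
; On BeginPlay it tests whether ValueA is greater than ValueB and prints "True" in green or "False" in red on screen.
; The other comparison operators sit in the graph as unconnected nodes, and the construction script is empty.
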(event EventBeginPlay
  (if (> (Variables|Default|GetValue_A) (Variables|Default|GetValue_B))
    (Development|PrintString "True" true true "(R=0.000000,G=1.000000,B=0.250000,A=1.000000)" 2e+01)
    (else
      (Development|PrintString "False" true true "(R=1.000000,G=0.000000,B=0.109699,A=1.000000)" 2e+01))))

(fn ConstructionScript)