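; A tutorial Actor Blueprint that demonstrates Blueprint variable types by printing them and applying them to the actor.
; On BeginPlay it prints a vector, waits, then moves the actor to that location and offsets its Cube component by the same vector.
; Disconnected example chains cover boolean, rotator, transform, numeric and text variables, including delayed rotation and transform changes and doubling a coin count.
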(event EventBeginPlay
  (bind _meshlocation (Variables|Default|GetMeshLocation))
  ;[0.15 0.15 0.15 0.5] Vector
  (Development|PrintString (Utilities|String|ToString(Vector) (Variables|Default|GetMeshLocation)) true true "(R=0.000000,G=0.660000,B=1.000000,A=1.000000)" 1e+01)
  (Utilities|FlowControl|Delay 5.0)
  (Transformation|SetActorLocation self _meshlocation false false)
  (Transformation|AddWorldOffset (Variables|Default|GetCube) _meshlocation false false))

(fn ConstructionScript)