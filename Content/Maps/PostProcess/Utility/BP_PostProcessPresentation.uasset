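; Utility actor that presents a post-process material alongside a configurable text label, apparently for showcasing effects in a map.
; The construction script applies the exposed text, size and color to a TextRender component.
; It also creates a dynamic material instance from a parent material and rebuilds the PostProcess component's settings with a post-process materials list.
; All setup happens at construction, with no active runtime events.
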(event EventBeginPlay)

(event Collision|EventActorBeginOverlap
  (params (OtherActor :type Actor%20Object%20Reference)))

(event EventTick
  (params (DeltaSeconds :type Float%20%28single-precision%29)))

(fn ConstructionScript
  (bind _textrender (Variables|Default|GetTextRender))
  (Rendering|Components|TextRender|SetText _textrender (Variables|Default|GetText))
  (Rendering|Components|TextRender|SetWorldSize _textrender (Variables|Default|GetTextSize))
  (Rendering|Components|TextRender|SetTextRenderColor _textrender (Variables|Default|GetTextColor))
  (Rendering|Material|CreateDynamicMaterialInstance (Variables|Default|GetParent) "None" "None" :!class /Script/Engine.KismetMaterialLibrary)
  (Variables|/Script/Engine.PostProcessComponent|SetSettings (Variables|Default|GetPostProcess) (Utilities|Struct|MakePostProcessSettings (Variables|Default|GetPost%20Process%20Materials))))