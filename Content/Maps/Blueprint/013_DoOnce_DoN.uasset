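; Demo Blueprint for the DoOnce and DoN flow nodes, using debug prints and a simple ammo counter.
; Key 1 prints through a DoOnce gate, which key 2 resets.
; Left mouse passes through a DoN limited by Ammo, printing the remaining count from RemainAmmo minus the DoN counter.
; R prints a reload message, restores RemainAmmo to Ammo and resets the DoN.
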(event EventBeginPlay
  (Variables|Default|SetRemainAmmo (Variables|Default|GetAmmo)))

(event Input|KeyboardEvents|R
  (params (Key :type Key%20Structure :default "None"))
  (bind _ammo (Variables|Default|GetAmmo))
  (:Pressed
    (Development|PrintString "Reload")
    (Variables|Default|SetRemainAmmo _ammo)
    (Utilities|FlowControl|DoN _ammo) ; enters at Reset
  ))

(event Input|MouseEvents|LeftMouseButton
  (params (Key :type Key%20Structure :default "None"))
  (:Pressed
    (bind _counter (Utilities|FlowControl|DoN (Variables|Default|GetAmmo))
      (:Exit
        (Development|PrintString (Utilities|String|Append "Ammo" (Utilities|String|ToString(Integer) (- (Variables|Default|GetRemainAmmo) _counter))))))))

(event Input|KeyboardEvents|1
  (params (Key :type Key%20Structure :default "None"))
  (:Pressed
    (Utilities|FlowControl|DoOnce false
      (:Completed
        (Development|PrintString "Hello" true true "(R=0.000000,G=0.660000,B=1.000000,A=1.000000)" 1e+01)))))

(event Input|KeyboardEvents|2
  (params (Key :type Key%20Structure :default "None"))
  (:Pressed
    (Utilities|FlowControl|DoOnce false) ; enters at Reset
  ))

(fn ConstructionScript)