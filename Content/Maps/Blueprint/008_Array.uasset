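; Array practice Blueprint that exercises basic operations on a Names array and prints results to screen.
; On BeginPlay it clears Names and prints the resulting length.
; Disconnected chains add a name and print the returned index, or print a Contains check against NewVar.
; Unused Random, Length and LastIndex nodes also remain in the graph, and the construction script is empty.
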(event EventBeginPlay
  (bind _names (Variables|Default|GetNames))
  (Utilities|Array|Clear _names)
  (Development|PrintString (Utilities|String|ToString(Integer) (Utilities|Array|Length _names)) true true "(R=0.000000,G=0.660000,B=1.000000,A=1.000000)" 1e+01))

(fn ConstructionScript)