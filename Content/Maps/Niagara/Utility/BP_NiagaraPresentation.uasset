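; BP_NiagaraPresentation is a display actor that presents either a Niagara system or a static mesh preview with a configurable text label.
; The Construction Script sets the label's text, size and color, then uses the NiagaraMesh flag to show the Niagara component with its assigned system or the mesh with its assigned material.
; The unused component is hidden, and all setup happens at construction, with no active event logic.
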(event EventBeginPlay)

(event Collision|EventActorBeginOverlap
  (params (OtherActor :type Actor%20Object%20Reference)))

(event EventTick
  (params (DeltaSeconds :type Float%20%28single-precision%29)))

(fn ConstructionScript
  (bind _previewmesh (Variables|Default|GetPreviewMesh))
  (Utilities|FlowControl|Sequence
    (:then_0
      (Rendering|Components|TextRender|SetText (Variables|Default|GetTextRender) (Variables|Default|GetText))
      (Rendering|Components|TextRender|SetWorldSize (Variables|Default|GetTextRender) (Variables|Default|GetTextSize))
      (Rendering|Components|TextRender|SetTextRenderColor (Variables|Default|GetTextRender) (Variables|Default|GetTextColor)))
    (:then_1
      (if (Variables|Default|GetNiagara/Mesh)
        (Rendering|SetVisibility _previewmesh false false)
        (else
          (Rendering|SetVisibility _previewmesh true false)
          (Rendering|Material|SetMaterial (Variables|Default|GetPreviewMesh) 0 (Variables|Default|GetMaterial))
          (Components|StaticMesh|SetStaticMesh (Variables|Default|GetPreviewMesh) (Variables|Default|GetPreview%20Mesh)))))
    (:then_2
      (if (Variables|Default|GetNiagara/Mesh)
        (Rendering|SetVisibility (Variables|Default|GetNiagara) true false)
        (Class|NiagaraComponent|SetAsset (Variables|Default|GetNiagara) (Variables|Default|GetNiagaraSystem) true)
        (else
          (Rendering|SetVisibility (Variables|Default|GetNiagara) false false))))))